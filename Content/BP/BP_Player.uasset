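; Player Blueprint that handles look input and confines the view to a limited yaw and pitch range around its starting control rotation.
; On BeginPlay, SetRotationLimits derives min and max angles from the initial rotation plus or minus horizontal and vertical limits.
; Turn and LookUp axis inputs add to the current angle, clamp it with ClampAngle and ClampAxis, then set player controller 0's control rotation directly.
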(event EventBeginPlay
  (CallFunction|SetRotationLimits))

(event Input|AxisEvents|InputAxisTurn
  (params (AxisValue :type Float%20%28single-precision%29))
  (bind _returnvalue (Pawn|GetControlRotation :!class /Script/Engine.Pawn))
  (Pawn|SetControlRotation (Game|GetPlayerController 0) (Math|Rotator|MakeRotator (.roll _returnvalue) (.pitch _returnvalue) (Class|KismetMathLibrary|ClampAxis (Math|Float|ClampAngle (+ AxisValue (.yaw _returnvalue)) (Variables|Default|GetMinYaw) (Variables|Default|GetMaxYaw))))))

(event Input|AxisEvents|InputAxisLookUp
  (params (AxisValue :type Float%20%28single-precision%29))
  (bind _returnvalue (Pawn|GetControlRotation :!class /Script/Engine.Pawn))
  (Pawn|SetControlRotation (Game|GetPlayerController 0) (Math|Rotator|MakeRotator (.roll _returnvalue) (Class|KismetMathLibrary|ClampAxis (Math|Float|ClampAngle (+ AxisValue (.pitch _returnvalue)) (Variables|Default|GetMinPitch) (Variables|Default|GetMaxPitch))) (.yaw _returnvalue))))

(fn ConstructionScript)

(fn SetRotationLimits
  (bind _returnvalue (Pawn|GetControlRotation :!class /Script/Engine.Pawn))
  (bind _horizontalrotlimit (Variables|Public|GetHorizontalRotLimit))
  (bind _verticalrotlimit (Variables|Public|GetVerticalRotLimit))
  (Variables|Default|SetMinYaw (- (.yaw _returnvalue) _horizontalrotlimit))
  (Variables|Default|SetMaxYaw (+ (.yaw _returnvalue) _horizontalrotlimit))
  (Variables|Default|SetMinPitch (- (.pitch _returnvalue) _verticalrotlimit))
  (Variables|Default|SetMaxPitch (+ (.pitch _returnvalue) _verticalrotlimit)))